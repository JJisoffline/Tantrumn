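; BP_HourOfCode_Character is a character Blueprint that prints jump debugging information.
; It prints velocity and records position on jumping, then prints straight-line distance travelled on landing.
; Tick detects the apex from a vertical velocity sign change and prints elapsed time, but the node setting JumpStartTime is disconnected.
; A Hold macro uses two gates and a retriggerable delay to distinguish Tap from Held input.
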(event `self.OnJumped`
  ;[1 1 1] Jump Time Debug
  ;[1 1 1] Jump Distance Debug
  (set `self.StartPosition` (`self.K2_GetActorLocation`))
  (`KismetSystemLibrary.PrintString` (`KismetStringLibrary.Conv_VectorToString` (`self.GetVelocity`)) true true (struct :`R` 1.0 :`B` 0.665464 :`A` 1.0) 10.0))

(event `self.OnLanded`
  (params (Hit :type "HitResult Structure (by ref)"))
  ;[1 1 1] Jump Time Debug
  ;[1 1 1] Jump Distance Debug
  (`KismetSystemLibrary.PrintString` "Jump Distance:" true true (struct :`R` 1.0 :`B` 0.665464 :`A` 1.0) 10.0)
  (`KismetSystemLibrary.PrintString` (`KismetStringLibrary.Conv_DoubleToString` (`KismetMathLibrary.VSize` (- (`self.K2_GetActorLocation`) (`self.StartPosition`)))) true true (struct :`R` 1.0 :`B` 0.665464 :`A` 1.0) 10.0))

(event `self.ReceiveTick`
  (params (DeltaSeconds :type "Float (single-precision)"))
  (bind (_returnvalue_x _returnvalue_y _returnvalue_z) (`KismetMathLibrary.BreakVector` (`self.GetVelocity`)))
  (bind (_lastvelocity_x _lastvelocity_y _lastvelocity_z) (`KismetMathLibrary.BreakVector` (`self.LastVelocity`)))
  ;[1 1 1] Velocity Debug
  (if (and (> _lastvelocity_z 0.0) (< _returnvalue_z 0.0))
    (`KismetSystemLibrary.PrintString` "Apex Time:" true true (struct :`R` 1.0 :`G` 0.920566 :`B` 0.201985 :`A` 1.0) 10.0)
    (`KismetSystemLibrary.PrintString` (`KismetStringLibrary.Conv_DoubleToString` (- (`GameplayStatics.GetTimeSeconds`) (`self.JumpStartTime`))) true true (struct :`R` 1.0 :`G` 0.874384 :`B` 0.21577 :`A` 1.0) 10.0))
  (set `self.LastVelocity` (`self.GetVelocity`)))

(fn `UserConstructionScript`)